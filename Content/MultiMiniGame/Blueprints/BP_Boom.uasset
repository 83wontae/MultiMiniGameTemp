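; BP_Boom is an explosive physics projectile that launches forward on spawn and explodes when it hits something.
; BeginPlay applies a large forward impulse to the Collision component.
; On hit it spawns a scaled explosion emitter, deals radial damage credited to its instigator's controller, and draws a debug sphere of the damage radius.
; It then hides itself, disables physics and collision, and destroys itself after a short timer delay.
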(event OnComponentHit(Collision)
  (params (HitComponent :type Primitive%20Component%20Object%20Reference) (OtherActor :type Actor%20Object%20Reference) (OtherComp :type Primitive%20Component%20Object%20Reference) (NormalImpulse :type Vector :default "0, 0, 0") (Hit :type Hit%20Result%20Structure%20%28by%20ref%29))
  (bind _location (Collision|BreakHitResult Hit))
  (CallFunction|ResHitBoom _location)
  (Game|Damage|ApplyRadialDamage 1e+02 _location (Variables|Default|GetDamage%20Radius) 0 0 self (Pawn|GetController (Variables|Actor|GetInstigator)) false "ECC_Visibility")
  (Rendering|Debug|DrawDebugSphere _location (Variables|Default|GetDamage%20Radius) 32 "(R=1.000000,G=0.000000,B=0.000000,A=1.000000)" 2e+01 2.0)
  (CallFunction|StartDestroy))

(event Custom|ResHitBoom
  (params (HitPoint :type Vector))
  (Effects|SpawnEmitteratLocation "/Game/StarterContent/Particles/P_Explosion.P_Explosion" HitPoint "0, 0, 0" "3.000000,3.000000,3.000000"))

(event EventBeginPlay
  (Physics|AddImpulse (Variables|Default|GetCollision) (* (Transformation|GetActorForwardVector) 1e+05) "None" false))

(fn ConstructionScript)

(fn StartDestroy
  (Rendering|SetActorHiddenInGame true)
  (Physics|SetSimulatePhysics (Variables|Default|GetCollision) false)
  (Collision|SetCollisionEnabled (Variables|Default|GetCollision) "NoCollision")
  (Utilities|Time|SetTimerbyFunctionName 0 "EventDestroyDelayEnd" 3.0))

(fn EventDestroyDelayEnd
  (Actor|DestroyActor))
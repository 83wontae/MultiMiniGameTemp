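; BP_MMGameMode is the game mode for a multiplayer minigame that splits joining players into attacker and defender roles.
; When a new player starts, the first one is stored as Attacker and possesses a BP_Attacker spawned at the "Attack" player start.
; While that Attacker reference is valid, every later player gets a BP_Defender spawned at the "Defend" player start.
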(event EventHandleStartingNewPlayer
  (params (NewPlayer :type Player%20Controller%20Object%20Reference))
  (|CallParentFunction NewPlayer)
  (Utilities|IsValid (Variables|Default|GetAttacker)
    (:Is%20Valid
      (bind _returnvalue (Game|SpawnActorfromClass "/Game/MultiMiniGame/GameMode/BP_Defender.BP_Defender_C" (Transformation|GetActorTransform (Class|GameModeBase|FindPlayerStart 0 "Defend")) "Undefined" "MultiplyWithRoot" 0 0))
      (Pawn|Possess NewPlayer _returnvalue))
    (:Is%20Not%20Valid
      (bind _output_get (Variables|Default|SetAttacker NewPlayer))
      (bind _returnvalue_2 (Game|SpawnActorfromClass "/Game/MultiMiniGame/GameMode/BP_Attacker.BP_Attacker_C" (Transformation|GetActorTransform (Class|GameModeBase|FindPlayerStart _output_get "Attack")) "Undefined" "MultiplyWithRoot" 0 0))
      (Pawn|Possess NewPlayer _returnvalue_2))))

(fn ConstructionScript)
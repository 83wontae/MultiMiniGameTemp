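; Spline actor that draws a path, such as a predicted projectile trajectory, as a chain of runtime-created spline mesh segments.
; Construction script lays fixed-length segments along the spline, clamping tangents to the section length.
; UpdateProjectilePath clears old meshes and points, rebuilds the spline from a predicted projectile trace, then adds one mesh per point-to-point span.
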(fn ConstructionScript
  (CallFunction|UpdateDrawSplineDistance))

(fn UpdateDrawSplinePoint
  (bind _spline (Variables|Default|GetSpline))
  (for _index (range 0 (Spline|GetNumberOfSplinePoints (Variables|Default|GetSpline)))
    (CallFunction|AddSplineMesh true (.Location (Spline|GetLocationandTangentatSplinePoint _spline _index "World")) (.Tangent (Spline|GetLocationandTangentatSplinePoint _spline _index "World")) (.Location (Spline|GetLocationandTangentatSplinePoint _spline (+ _index 1) "World")) (.Tangent (Spline|GetLocationandTangentatSplinePoint _spline (+ _index 1) "World")))))

(fn UpdateProjectilePath
  (params (Start%20Location :type Vector) (Launch%20Velocity :type Vector))
  (CallFunction|ClearSplineMesh)
  (bind _predictresult (Class|GameplayStatics|BlueprintPredictProjectilePathAdvanced (Utilities|Struct|MakePredictProjectilePathParams Start%20Location Launch%20Velocity false 1.0 1.0 true "ECC_Visibility" (Utilities|Array|MakeArray "ObjectTypeQuery1" "ObjectTypeQuery2"))))
  (for _array_element (.PathData (Utilities|Struct|BreakPredictProjectilePathResult _predictresult))
    (Spline|AddSplinePoint (Variables|Default|GetSpline) (.Location (Utilities|Struct|BreakPredictProjectilePathPointData _array_element)) "World" true))
  (CallFunction|UpdateDrawSplinePoint))

(fn AddSplineMesh
  (params (bManualAttachment :type Boolean) (StartPos :type Vector) (StartTangent :type Vector) (EndPos :type Vector) (EndTangent :type Vector))
  (bind _returnvalue (AddComponent|AddSplineMeshComponent bManualAttachment))
  (Utilities|Array|Add (Variables|Default|GetSplineMeshComps) _returnvalue)
  (Transformation|SetMobility _returnvalue "Movable")
  (Components|StaticMesh|SetStaticMesh _returnvalue (Variables|Default|GetSplineMesh))
  (SplineMesh|SetForwardAxis _returnvalue "X" false)
  (SplineMesh|SetStartandEnd _returnvalue StartPos StartTangent EndPos EndTangent true :!class /Script/Engine.SplineMeshComponent))

(fn ClearSplineMesh
  (bind _splinemeshcomps (Variables|Default|GetSplineMeshComps))
  (Components|DestroyComponent _splinemeshcomps)
  (Utilities|Array|Clear _splinemeshcomps)
  (Spline|ClearSplinePoints (Variables|Default|GetSpline) true))

(fn UpdateDrawSplineDistance
  (bind _spline (Variables|Default|GetSpline))
  (for _index (range 0 (Math|Float|Truncate (/ (Spline|GetSplineLength (Variables|Default|GetSpline)) (Variables|Default|GetSectionLength))))
    (CallFunction|AddSplineMesh true (Spline|GetLocationatDistanceAlongSpline _spline (* _index (Variables|Default|GetSectionLength)) "World") (Math|Vector|ClampVectorSize (Spline|GetTangentatDistanceAlongSpline _spline (* _index (Variables|Default|GetSectionLength)) "World") 0.0 (Variables|Default|GetSectionLength)) (Spline|GetLocationatDistanceAlongSpline _spline (* (+ _index 1) (Variables|Default|GetSectionLength)) "World") (Math|Vector|ClampVectorSize (Spline|GetTangentatDistanceAlongSpline _spline (* (+ _index 1) (Variables|Default|GetSectionLength)) "World") 0.0 (Variables|Default|GetSectionLength)))))